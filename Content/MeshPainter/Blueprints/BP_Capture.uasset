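; BP_Capture is a Mesh Painter Blueprint that initializes the shared parameters and render target for an orthographic scene capture.
; On BeginPlay it writes the capture's ortho width and the UnwrapLocation into MPC_Global as CaptureSize and UnwrapLocation, making them available to materials.
; After a short delay it clears RT_Capture to opaque black.
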(event `self.ReceiveBeginPlay`
  (`self.InitializeParameters`))

(fn `UserConstructionScript`)